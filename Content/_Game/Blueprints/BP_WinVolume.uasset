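; BP_WinVolume is a trigger volume that completes the level when the player character overlaps its Cylinder component.
; It pauses the game mode's timer and the game, then saves the win through BP_GameInstance.
; It replaces all widgets with WBP_LevelCompleteScreen, switches to UI-only input with a visible cursor, calls CallWin and destroys the LevelMusic actor.
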(event OnComponentBeginOverlap(Cylinder)
  (params (OverlappedComponent :type Primitive%20Component%20Object%20Reference) (OtherActor :type Actor%20Object%20Reference) (OtherComp :type Primitive%20Component%20Object%20Reference) (OtherBodyIndex :type Integer) (bFromSweep :type Boolean) (SweepResult :type Hit%20Result%20Structure%20%28by%20ref%29))
  (bind _returnvalue (Game|GetPlayerController 0))
  (if (== OtherActor (Game|GetPlayerCharacter 0))
    (bind _asbp_first_person_game_mode (Utilities|Casting|CastToBP_FirstPersonGameMode (Game|GetGameMode)))
    (Default|PauseTimer _asbp_first_person_game_mode)
    (Game|SetGamePaused true)
    (bind _asbp_game_instance (Utilities|Casting|CastToBP_GameInstance (Game|GetGameInstance)))
    (Default|LevelWinSave _asbp_game_instance)
    (Viewport|RemoveAllWidgets)
    (bind _returnvalue_2 (UserInterface|CreateWidget "/Game/_Game/UI/WBP_LevelCompleteScreen.WBP_LevelCompleteScreen_C" _returnvalue))
    (UserInterface|Viewport|AddtoViewport _returnvalue_2 0)
    (Input|SetInputModeUIOnly _returnvalue 0 "DoNotLock" false)
    (Variables|/Script/Engine.PlayerController|SetbShowMouseCursor _returnvalue true)
    (Default|CallWin)
    (Actor|DestroyActor (Variables|Default|GetLevelMusic))))

(event EventBeginPlay)

(event Collision|EventActorBeginOverlap
  (params (OtherActor :type Actor%20Object%20Reference)))

(event EventTick
  (params (DeltaSeconds :type Float%20%28single-precision%29)))

(fn ConstructionScript)