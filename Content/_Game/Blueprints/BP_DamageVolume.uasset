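; BP_DamageVolume is a hazard volume that tracks whether the player is inside and whether it can currently damage, without applying damage itself.
; Capsule overlaps with the player character set the Overlap flag.
; If DoesOnAndOff is set, a looping timer toggles CanDamage along with the visibility of four particle systems.
; Each overlap change or toggle fires StatusChange, presumably a dispatcher for listeners that handle the damage.
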(event OnComponentBeginOverlap(Capsule)
  (params (OverlappedComponent :type Primitive%20Component%20Object%20Reference) (OtherActor :type Actor%20Object%20Reference) (OtherComp :type Primitive%20Component%20Object%20Reference) (OtherBodyIndex :type Integer) (bFromSweep :type Boolean) (SweepResult :type Hit%20Result%20Structure%20%28by%20ref%29))
  (if (== OtherActor (Game|GetPlayerCharacter 0))
    (Variables|Default|SetOverlap true)
    (Default|CallStatusChange)))

(event OnComponentEndOverlap(Capsule)
  (params (OverlappedComponent :type Primitive%20Component%20Object%20Reference) (OtherActor :type Actor%20Object%20Reference) (OtherComp :type Primitive%20Component%20Object%20Reference) (OtherBodyIndex :type Integer))
  (if (== OtherActor (Game|GetPlayerCharacter 0))
    (Variables|Default|SetOverlap false)
    (Default|CallStatusChange)))

(event EventBeginPlay
  (if (Variables|Default|GetDoesOnAndOff)
    (Utilities|Time|SetTimerbyFunctionName 0 "OnAndOff" 2.0 true)))

(event Collision|EventActorBeginOverlap
  (params (OtherActor :type Actor%20Object%20Reference)))

(event EventTick
  (params (DeltaSeconds :type Float%20%28single-precision%29)))

(fn ConstructionScript)

(fn OnandOff
  (if (Variables|Default|GetCanDamage)
    (Variables|Default|SetCanDamage false)
    (Rendering|SetVisibility (Variables|Default|GetParticleSystem) false false)
    (Rendering|SetVisibility (Variables|Default|GetParticleSystem2) false false)
    (Rendering|SetVisibility (Variables|Default|GetParticleSystem1) false false)
    (Rendering|SetVisibility (Variables|Default|GetParticleSystem3) false false)
    (else
      (Variables|Default|SetCanDamage true)
      (Rendering|SetVisibility (Variables|Default|GetParticleSystem) true false)
      (Rendering|SetVisibility (Variables|Default|GetParticleSystem2) true false)
      (Rendering|SetVisibility (Variables|Default|GetParticleSystem1) true false)
      (Rendering|SetVisibility (Variables|Default|GetParticleSystem3) true false)))
  (Default|CallStatusChange))