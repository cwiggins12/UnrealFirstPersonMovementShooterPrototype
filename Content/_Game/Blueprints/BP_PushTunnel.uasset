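; BP_PushTunnel is a tunnel actor that launches the player along its forward vector when a linked button is pressed.
; It binds to ButtonRef's press event and fires only while the player overlaps the Cylinder volume.
; The launch is a velocity-change impulse scaled by LaunchMult, with a whoosh sound.
; On BeginPlay, an otherwise unused line trace draws a persistent white debug line toward the button.
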(event OnComponentBeginOverlap(Cylinder)
  (params (OverlappedComponent :type Primitive%20Component%20Object%20Reference) (OtherActor :type Actor%20Object%20Reference) (OtherComp :type Primitive%20Component%20Object%20Reference) (OtherBodyIndex :type Integer) (bFromSweep :type Boolean) (SweepResult :type Hit%20Result%20Structure%20%28by%20ref%29))
  (if (== OtherActor (Game|GetPlayerCharacter 0))
    (Variables|Default|SetCanPush true)))

(event OnComponentEndOverlap(Cylinder)
  (params (OverlappedComponent :type Primitive%20Component%20Object%20Reference) (OtherActor :type Actor%20Object%20Reference) (OtherComp :type Primitive%20Component%20Object%20Reference) (OtherBodyIndex :type Integer))
  (if (== OtherActor (Game|GetPlayerCharacter 0))
    (Variables|Default|SetCanPush false)))

(event Custom|OnButtonPress
  (if (Variables|Default|GetCanPush)
    (Physics|AddImpulse (Variables|/Script/Engine.Character|GetCharacterMovement (Game|GetPlayerCharacter 0)) (* (Transformation|GetActorForwardVector) (Variables|Default|GetLaunchMult)) true)
    (Audio|PlaySoundatLocation "/Game/_Game/Audio/WhooshSFX_Cue.WhooshSFX_Cue" (Transformation|GetActorLocation) "0, 0, 0" 1.0 1.0 0.0 0 0 0 0)))

(event EventBeginPlay
  (EventDispatchers|BindEventtoButtonPressed (Variables|Default|GetButtonRef) (delegate Custom|OnButtonPress))
  (Collision|LineTraceByChannel (Transformation|GetActorLocation) (Transformation|GetActorLocation (Variables|Default|GetButtonRef)) "TraceTypeQuery2" false 0 "Persistent" true "(R=1.000000,G=1.000000,B=1.000000,A=1.000000)" "(R=1.000000,G=1.000000,B=1.000000,A=1.000000)"))

(fn ConstructionScript)