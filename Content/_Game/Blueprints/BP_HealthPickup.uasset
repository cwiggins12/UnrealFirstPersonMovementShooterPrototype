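; BP_HealthPickup is a pickup that restores the player's health when touched and then destroys itself.
; Its Collider overlap handler responds only to player pawn 0 and reads Health and MaxHealth from that pawn's BPC_HealthSystem, ignoring the touch when they are equal.
; Healing goes through ApplyDamage with HealAmount as the base damage, rather than a dedicated heal call.
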(event OnComponentBeginOverlap(Collider)
  (params (OverlappedComponent :type Primitive%20Component%20Object%20Reference) (OtherActor :type Actor%20Object%20Reference) (OtherComp :type Primitive%20Component%20Object%20Reference) (OtherBodyIndex :type Integer) (bFromSweep :type Boolean) (SweepResult :type Hit%20Result%20Structure%20%28by%20ref%29))
  (bind _returnvalue (Game|Player|GetPlayerPawn 0))
  (bind _returnvalue_2 (Actor|GetComponentbyClass _returnvalue "/Game/_Game/Blueprints/Component/BPC_HealthSystem.BPC_HealthSystem_C"))
  (if (== OtherActor _returnvalue)
    (if (not (== (Variables|/Game/_Game/Blueprints/Component/BPC_HealthSystem.BPC_HealthSystem_C|GetHealth _returnvalue_2) (Variables|/Game/_Game/Blueprints/Component/BPC_HealthSystem.BPC_HealthSystem_C|GetMaxHealth _returnvalue_2)))
      (Game|Damage|ApplyDamage _returnvalue (Variables|Default|GetHealAmount) 0 0)
      (Actor|DestroyActor))))

(event EventBeginPlay)

(event Collision|EventActorBeginOverlap
  (params (OtherActor :type Actor%20Object%20Reference)))

(event EventTick
  (params (DeltaSeconds :type Float%20%28single-precision%29)))

(fn ConstructionScript)