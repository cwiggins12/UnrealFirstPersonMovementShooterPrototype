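; BP_DamageActivatedButton is a button that fires its ButtonPressed event when damage depletes its health component.
; On the kill callback it disables damage, swaps to the pressed mesh and calls ButtonPressed.
; After a Cooldown delay it refills health, plays a ready sound, re-enables damage and shows the unpressed mesh, so it can trigger again.
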(event Custom|OnKilled
  (bind _bpc_healthsystem (Variables|Default|GetBPC_HealthSystem))
  (Variables|Actor|SetbCanBeDamaged false)
  (Rendering|SetVisibility (Variables|Default|GetPressedMesh) true false)
  (Rendering|SetVisibility (Variables|Default|GetUnpressedMesh) false false)
  (Default|CallButtonPressed)
  (Utilities|FlowControl|Delay (Variables|Default|GetCooldown))
  (Variables|/Game/_Game/Blueprints/Component/BPC_HealthSystem.BPC_HealthSystem_C|SetHealth _bpc_healthsystem (Variables|/Game/_Game/Blueprints/Component/BPC_HealthSystem.BPC_HealthSystem_C|GetMaxHealth _bpc_healthsystem))
  (Audio|PlaySoundatLocation "/Game/_Game/Audio/ButtonReadySFX_Cue.ButtonReadySFX_Cue" (Transformation|GetActorLocation) "0, 0, 0" 1.0 1.0 0.0 0 0 0 0)
  (Variables|Actor|SetbCanBeDamaged true)
  (Rendering|SetVisibility (Variables|Default|GetPressedMesh) false false)
  (Rendering|SetVisibility (Variables|Default|GetUnpressedMesh) true false))

(event EventBeginPlay
  (EventDispatchers|BindEventtoOnKilled (Variables|Default|GetBPC_HealthSystem) (delegate Custom|OnKilled)))

(fn ConstructionScript)