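; BP_Door is a door actor that opens and closes when its referenced button is pressed.
; On BeginPlay it binds OpenAndClose to the button's pressed event and runs a line trace to the button, which only draws a persistent debug line.
; OpenAndClose plays the open sound and lowers the Door component, pauses briefly, then plays the close sound and raises it, with separate down and up durations.
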(event Custom|OpenAndClose
  (bind _returnvalue (Transformation|GetActorLocation))
  (bind _door (Variables|Default|GetDoor))
  (Audio|PlaySoundatLocation "/Game/_Game/Audio/DoorOpenSFX_Cue.DoorOpenSFX_Cue" _returnvalue "0, 0, 0" 1.0 1.0 0.0 0 0 0 0)
  (Components|MoveComponentTo _door "0.000000,0.000000,-200.000000" "0, 0, 0" false false (Variables|Default|GetMoveDownTime) false)
  (Utilities|FlowControl|Delay 0.2)
  (Audio|PlaySoundatLocation "/Game/_Game/Audio/DoorCloseSFX_Cue.DoorCloseSFX_Cue" _returnvalue "0, 0, 0" 1.0 1.0 0.0 0 0 0 0)
  (Components|MoveComponentTo _door "0.000000,0.000000,100.000000" "0, 0, 0" false false (Variables|Default|GetMoveUpTime) false))

(event EventBeginPlay
  (EventDispatchers|BindEventtoButtonPressed (Variables|Default|GetButtonRef) (delegate Custom|OpenAndClose))
  (Collision|LineTraceByChannel (Transformation|GetActorLocation) (Transformation|GetActorLocation (Variables|Default|GetButtonRef)) "TraceTypeQuery2" false 0 "Persistent" true "(R=1.000000,G=1.000000,B=1.000000,A=1.000000)" "(R=1.000000,G=1.000000,B=1.000000,A=1.000000)"))

(fn ConstructionScript)