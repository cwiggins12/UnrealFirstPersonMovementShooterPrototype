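; Dash component that gates dash use and tracks its cooldown, leaving the movement itself to other code.
; StartDash succeeds only when not dashing and available, then zeroes the charge value and broadcasts ChangeInDashValue.
; StartCooldown unpauses a looping timer created paused at BeginPlay, which refills the normalized value and broadcasts each tick.
; At full charge it pauses the timer, re-enables dashing and plays a sound at the player pawn.
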(event EventBeginPlay
  (Variables|Default|SetCooldownTickAmount 1.0)
  (bind _returnvalue (Utilities|Time|SetTimerbyFunctionName 0 "CooldownTick" (Variables|Default|GetCooldownTickMod) true))
  (bind _output_get (Variables|Default|SetCooldownTimer _returnvalue))
  (Utilities|Time|PauseTimerbyHandle _output_get))

(event EventTick
  (params (DeltaSeconds :type Float%20%28single-precision%29)))

(fn StartDash
  (if (Variables|Default|GetIsDashing)
    _
    (elif (Variables|Default|GetCanDash)
      (Variables|Default|SetCanDash false)
      (Variables|Default|SetCooldownTickAmount 0.0)
      (Default|CallChangeinDashValue)
      (return true)
      (else
        _)))
  (return false))

(fn StopDash
  (Variables|Default|SetIsDashing false)
  (Variables|Default|SetOnCooldown true))

(fn StartCooldown
  (Variables|Default|SetOnCooldown true)
  (Utilities|Time|UnpauseTimerbyHandle (Variables|Default|GetCooldownTimer)))

(fn StopCooldown
  (Utilities|Time|PauseTimerbyHandle (Variables|Default|GetCooldownTimer))
  (Variables|Default|SetOnCooldown false)
  (Variables|Default|SetCanDash true)
  (Audio|PlaySoundatLocation "/Game/_Game/Audio/DashCooldown_Cue.DashCooldown_Cue" (Transformation|GetActorLocation (Game|Player|GetPlayerPawn 0)) "0, 0, 0" 1.0 1.0 0.0 0 0 0 0))

(fn CooldownTick
  (bind _output_get (Variables|Default|SetCooldownTickAmount (Math|Float|Clamp(Float) (+ (/ (Variables|Default|GetCooldownTickMod) (Variables|Default|GetDashCooldown)) (Variables|Default|GetCooldownTickAmount)))))
  (Default|CallChangeinDashValue)
  (if (>= _output_get 1.0)
    (CallFunction|StopCooldown)))