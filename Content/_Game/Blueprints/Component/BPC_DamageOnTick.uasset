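; Actor component that deals repeated damage to the player while its owning BP_DamageVolume is overlapped and allowed to damage.
; On BeginPlay it casts its owner to BP_DamageVolume and binds to that volume's status change event.
; The status check applies damage at once and starts a looping timer, or clears the timer when either condition fails.
; Damage always targets player character 0, regardless of what overlaps.
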(event EventBeginPlay
  (bind _output_get (Variables|Default|SetOwner (Components|GetOwner)))
  (bind _asbp_damage_volume (Utilities|Casting|CastToBP_DamageVolume _output_get))
  (bind _output_get_2 (Variables|Default|SetOwnerAsDamageVolume _asbp_damage_volume))
  (EventDispatchers|BindEventtoStatusChange _output_get_2 (EventDispatchers|CreateEvent :!event CanWeDamageonStatusChange)))

(fn DoDamage
  (Game|Damage|ApplyDamage (Game|GetPlayerCharacter 0) (Variables|Default|GetDamageAmount) 0 0))

(fn CanWeDamageonStatusChange
  (bind _ownerasdamagevolume (Variables|Default|GetOwnerAsDamageVolume))
  (if (and (Variables|/Game/_Game/Blueprints/BP_DamageVolume.BP_DamageVolume_C|GetOverlap _ownerasdamagevolume) (Variables|/Game/_Game/Blueprints/BP_DamageVolume.BP_DamageVolume_C|GetCanDamage _ownerasdamagevolume))
    (CallFunction|DoDamage)
    (Utilities|Time|SetTimerbyFunctionName 0 "DoDamage" 0.1 true)
    (else
      (Utilities|Time|ClearTimerbyFunctionName 0 "DoDamage"))))