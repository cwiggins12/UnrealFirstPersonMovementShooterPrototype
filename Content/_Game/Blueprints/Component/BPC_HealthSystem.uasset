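; Reusable health component that gives its owning actor hit points, damage and healing feedback, and death handling.
; On BeginPlay it fills health to max and binds to the owner's OnTakeAnyDamage.
; Each change clamps health and plays sound and Niagara FX, treating zero or negative damage as healing and shaking the camera for player hits.
; It broadcasts change, heal and killed events for other logic to react to.
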(event Custom|ChangeInHealth
  (params (DamagedActor :type Actor%20Object%20Reference) (Damage :type Float%20%28single-precision%29) (DamageType :type Damage%20Type%20Object%20Reference) (InstigatedBy :type Controller%20Object%20Reference) (DamageCauser :type Actor%20Object%20Reference))
  (bind _owner (Variables|Default|GetOwner))
  (Variables|Default|SetHealth (Math|Float|Clamp(Float) (- (Variables|Default|GetHealth) Damage) 0.0 (Variables|Default|GetMaxHealth)))
  (if (> Damage 0.0)
    (CallFunction|PlayDamageFX)
    (if (== _owner (Game|GetPlayerCharacter 0))
      (Camera|PlayWorldCameraShake "/Game/_Game/Blueprints/BP_DamagedCamShake.BP_DamagedCamShake_C" (Transformation|GetActorLocation _owner) 0.0 1.5e+03))
    (else
      (CallFunction|PlayHealFX)
      (Default|CallOnHeal)))
  (Default|CallOnChangeinHealth Damage)
  (if (<= (Variables|Default|GetHealth) 0.0)
    (CallFunction|PlayKillFX)
    (Default|CallOnKilled)))

(event EventBeginPlay
  (Variables|Default|SetOwner (Components|GetOwner))
  (Variables|Default|SetHealth (Variables|Default|GetMaxHealth))
  (EventDispatchers|BindEventtoOnTakeAnyDamage (Variables|Default|GetOwner) (EventDispatchers|CreateEvent :!event Custom|ChangeInHealth)))

(fn PlayKillFX
  (bind _killsound (Variables|Default|GetKillSound))
  (bind _owner (Variables|Default|GetOwner))
  (bind _returnvalue (Transformation|GetActorLocation _owner))
  (Utilities|IsValid _killsound
    (:Is%20Valid
      (Audio|PlaySoundatLocation _killsound _returnvalue "0, 0, 0" 1.0 1.0 0.0 0 0 0 0))
    (:Is%20Not%20Valid
      _))
  (Utilities|IsValid _owner
    (:Is%20Valid
      (Niagara|SpawnSystematLocation (Variables|Default|GetKillParticles) _returnvalue))))

(fn PlayDamageFX
  (bind _owner (Variables|Default|GetOwner))
  (bind _damagedsound (Variables|Default|GetDamagedSound))
  (bind _damagedparticles (Variables|Default|GetDamagedParticles))
  (bind _returnvalue (Transformation|GetActorLocation _owner))
  (Utilities|IsValid _damagedsound
    (:Is%20Valid
      (Audio|PlaySoundatLocation _damagedsound _returnvalue "0, 0, 0" 1.0 1.0 0.0 0 0 0 0))
    (:Is%20Not%20Valid
      _))
  (Utilities|IsValid _damagedparticles
    (:Is%20Valid
      (Niagara|SpawnSystematLocation _damagedparticles _returnvalue))))

(fn PlayHealFX
  (bind _healsound (Variables|Default|GetHealSound))
  (bind _healparticles (Variables|Default|GetHealParticles))
  (bind _owner (Variables|Default|GetOwner))
  (bind _returnvalue (Transformation|GetActorLocation _owner))
  (Utilities|IsValid _healsound
    (:Is%20Valid
      (Audio|PlaySoundatLocation _healsound _returnvalue "0, 0, 0" 1.0 1.0 0.0 0 0 0 0))
    (:Is%20Not%20Valid
      _))
  (Utilities|IsValid _healparticles
    (:Is%20Valid
      (Niagara|SpawnSystematLocation _healparticles _returnvalue))))