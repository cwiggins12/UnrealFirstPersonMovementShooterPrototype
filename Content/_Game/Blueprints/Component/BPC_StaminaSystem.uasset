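; Stamina component that tracks a stamina pool, starting full and refilling over time after it is spent.
; SpendStamina subtracts a positive amount, clamped at zero, then pauses regeneration for a set duration, which restarts with each spend.
; A single looping timer runs TickStamina to add regen scaled by tick interval.
; That timer is paused and unpaused rather than recreated, and pauses itself once stamina is full.
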(event EventBeginPlay
  (Variables|Default|SetStamina (Variables|Default|GetMaxStamina))
  (bind _returnvalue (Utilities|Time|SetTimerbyFunctionName 0 "TickStamina" (Variables|Default|GetStaminaTickFrequency) true))
  (bind _output_get (Variables|Default|SetStaminaTickTimer _returnvalue))
  (Utilities|Time|PauseTimerbyHandle _output_get))

(fn TickStamina
  (bind _maxstamina (Variables|Default|GetMaxStamina))
  (Variables|Default|SetStamina (Math|Float|Clamp(Float) (+ (Variables|Default|GetStamina) (* (Variables|Default|GetStaminaRegenPerSec) (Variables|Default|GetStaminaTickFrequency))) 0.0 _maxstamina))
  (if (== (Variables|Default|GetStamina) _maxstamina)
    (CallFunction|StopTickStamina)))

(fn SpendStamina
  (params (Amount :type Float%20%28double-precision%29))
  (if (> Amount 0.0)
    (Variables|Default|SetStamina (Math|Float|Clamp(Float) (- (Variables|Default|GetStamina) Amount) 0.0 (Variables|Default|GetMaxStamina)))
    (CallFunction|PauseTickStamina (Variables|Default|GetStaminaSpendPauseDuration))))

(fn PauseTickStamina
  (params (Duration :type Float%20%28double-precision%29))
  (Utilities|Time|PauseTimerbyHandle (Variables|Default|GetStaminaTickTimer))
  (if (> Duration 0.0)
    (Utilities|Time|SetTimerbyFunctionName 0 "StartTickStamina" Duration)
    (else
      (CallFunction|StartTickStamina))))

(fn StartTickStamina
  (Utilities|Time|UnpauseTimerbyHandle (Variables|Default|GetStaminaTickTimer)))

(fn StopTickStamina
  (Utilities|Time|PauseTimerbyHandle (Variables|Default|GetStaminaTickTimer)))