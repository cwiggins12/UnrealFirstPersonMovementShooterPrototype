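; BP_ExtraJumpButton is a button that grants the first-person character an extra jump when its health component is killed.
; On kill it shows as pressed, disables collision, increments the character's extra jump count and records that count.
; Each jump-subtract event from the character counts the record down; at zero the button restores health, collision and visuals with a ready sound.
; An impulse-and-boing chain is left unconnected.
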(event Custom|OnKilled
  (bind _fpcharacterref (Variables|Default|GetFPCharacterRef))
  (Variables|Default|SetCanBeDamaged false)
  (Collision|SetCollisionEnabled (Variables|Default|GetBox) "NoCollision")
  (Rendering|SetVisibility (Variables|Default|GetPressedMesh) true false)
  (Rendering|SetVisibility (Variables|Default|GetUnpressedMesh) false false)
  (Rendering|Components|TextRender|SetTextRenderColor (Variables|Default|GetTextRender) (Math|Color|MakeColor 0 0 0 100))
  (bind _result (Math|Integer|IncrementInt (Variables|/Game/FirstPerson/Blueprints/BP_FirstPersonCharacter.BP_FirstPersonCharacter_C|GetExtraJumpAmount _fpcharacterref))
    (:%20%20
      (Variables|Default|SetExtraJumpsOnPress _result)
      (Default|CallExtraJumpAmountAdd _fpcharacterref))))

(event Custom|OnJumpAmountSub
  (bind _bpc_healthsystem (Variables|Default|GetBPC_HealthSystem))
  (if (not (Variables|Default|GetCanBeDamaged))
    (bind _result (Math|Integer|DecrementInt (Variables|Default|GetExtraJumpsOnPress))
      (:%20%20
        (if (== _result 0)
          (Variables|Actor|SetbCanBeDamaged true)
          (Variables|/Game/_Game/Blueprints/Component/BPC_HealthSystem.BPC_HealthSystem_C|SetHealth _bpc_healthsystem (Variables|/Game/_Game/Blueprints/Component/BPC_HealthSystem.BPC_HealthSystem_C|GetMaxHealth _bpc_healthsystem))
          (Audio|PlaySoundatLocation "/Game/_Game/Audio/ButtonReadySFX_Cue.ButtonReadySFX_Cue" (Transformation|GetActorLocation) "0, 0, 0" 1.0 1.0 0.0 0 0 0 0)
          (Collision|SetCollisionEnabled (Variables|Default|GetBox) "QueryAndPhysics")
          (Rendering|SetVisibility (Variables|Default|GetPressedMesh) false false)
          (Rendering|SetVisibility (Variables|Default|GetUnpressedMesh) true false)
          (Rendering|Components|TextRender|SetTextRenderColor (Variables|Default|GetTextRender) (Math|Color|MakeColor 255 255 255 255)))))))

(event EventBeginPlay
  (bind _asbp_first_person_character (Utilities|Casting|CastToBP_FirstPersonCharacter (Game|GetPlayerCharacter 0)))
  (bind _output_get (Variables|Default|SetFPCharacterRef _asbp_first_person_character))
  (EventDispatchers|BindEventtoExtraJumpAmountSub _output_get (delegate Custom|OnJumpAmountSub))
  (EventDispatchers|BindEventtoOnKilled (Variables|Default|GetBPC_HealthSystem) (delegate Custom|OnKilled)))

(fn ConstructionScript)